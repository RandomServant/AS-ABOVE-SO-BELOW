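; Vacuum cleaner actor that moves along with the player character and respawns when its HP runs out.
; Each tick it adds the player's horizontal movement delta to its own position and sets its yaw to the player's negated control yaw.
; At zero HP it plays a burst and boom, returns to its start, calls Die on the player and resets HP.
; BeginPlay also creates the trash-count widget and enables custom depth on the mesh.
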(event EventTick
  (params (DeltaSeconds :type Float%20%28single-precision%29))
  (bind _returnvalue (Transformation|GetActorLocation))
  (if (<= (Variables|Default|GetHP) 0.0)
    (Variables|Default|SetCharacterLocation (Math|Vector|MakeVector (.x (Transformation|GetActorLocation (stale _asbp_first_person_controller))) (.y (Transformation|GetActorLocation (stale _asbp_first_person_controller))) 0.0))
    (CallFunction|Dead)
    (else
      (bind _asbp_first_person_controller (Utilities|Casting|CastToBP_FirstPersonController (Game|GetPlayerCharacter 0)))
      (Transformation|SetActorRotation (Math|Rotator|MakeRotator 0.0 0.0 (* (.yaw (Pawn|GetControlRotation _asbp_first_person_controller :!class /Script/Engine.Pawn)) -1.0)))
      (Transformation|SetActorLocation (Math|Vector|MakeVector (+ (.x _returnvalue) (- (.x (Transformation|GetActorLocation _asbp_first_person_controller)) (.x (Variables|Default|GetCharacterLocation)))) (+ (.y _returnvalue) (- (.y (Transformation|GetActorLocation _asbp_first_person_controller)) (.y (Variables|Default|GetCharacterLocation)))) (.z _returnvalue)) false false)
      (Variables|Default|SetCharacterLocation (Math|Vector|MakeVector (.x (Transformation|GetActorLocation _asbp_first_person_controller)) (.y (Transformation|GetActorLocation _asbp_first_person_controller)) 0.0)))))

(event EventBeginPlay
  (bind _asbp_first_person_controller (Utilities|Casting|CastToBP_FirstPersonController (Game|GetPlayerCharacter 0)))
  (Variables|Default|SetCharacterLocation (Math|Vector|MakeVector (.x (Transformation|GetActorLocation _asbp_first_person_controller)) (.y (Transformation|GetActorLocation _asbp_first_person_controller)) 0.0))
  (bind _returnvalue (UserInterface|CreateWidget "/Game/Assets/CountOfTrash/CountOfTrash.CountOfTrash_C"))
  (UserInterface|Viewport|AddtoViewport _returnvalue 0)
  (Variables|Default|SetStartPosition (Transformation|GetActorLocation))
  (Rendering|SetRenderCustomDepth (Variables|Character|GetMesh) true))

(fn ConstructionScript)

(fn Dead
  (bind _returnvalue (Transformation|GetActorLocation))
  (Effects|SpawnEmitteratLocation "/Game/Levels/Sequence/Particals/Burst.Burst" _returnvalue)
  (Audio|PlaySoundatLocation "/Game/Music/Boom_Cue.Boom_Cue" _returnvalue "0, 0, 0" 1.0 1.0 0.0 0 0 0)
  (bind _asbp_first_person_controller (Utilities|Casting|CastToBP_FirstPersonController (Game|GetPlayerCharacter 0)))
  (Transformation|SetActorLocation (Variables|Default|GetStartPosition) false false)
  (Default|Die _asbp_first_person_controller)
  (Variables|Default|SetHP 1e+02))