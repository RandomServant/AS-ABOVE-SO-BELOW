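; BP_PushBox is a physics-simulated pushable cube that resets when the player dies.
; Overlaps with the X and Y collision components toggle IsPushing on BP_FirstPersonController.
; A Sphere overlap toggles the cube's custom depth rendering as a proximity highlight.
; Tick polls player Health and, while it is zero or below, zeroes the cube's linear velocity and returns it to its BeginPlay location.
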(event OnComponentBeginOverlap(YCollision)
  (params (OverlappedComponent :type Primitive%20Component%20Object%20Reference) (OtherActor :type Actor%20Object%20Reference) (OtherComp :type Primitive%20Component%20Object%20Reference) (OtherBodyIndex :type Integer) (bFromSweep :type Boolean) (SweepResult :type Hit%20Result%20Structure%20%28by%20ref%29))
  ;[1 1 1] Y
  (bind _asbp_first_person_controller (Utilities|Casting|CastToBP_FirstPersonController OtherActor))
  (Variables|/Game/Character/BP_FirstPersonController.BP_FirstPersonController_C|SetIsPushing? _asbp_first_person_controller true))

(event OnComponentEndOverlap(YCollision)
  (params (OverlappedComponent :type Primitive%20Component%20Object%20Reference) (OtherActor :type Actor%20Object%20Reference) (OtherComp :type Primitive%20Component%20Object%20Reference) (OtherBodyIndex :type Integer))
  ;[1 1 1] Y
  (bind _asbp_first_person_controller (Utilities|Casting|CastToBP_FirstPersonController OtherActor))
  (Variables|/Game/Character/BP_FirstPersonController.BP_FirstPersonController_C|SetIsPushing? _asbp_first_person_controller false))

(event OnComponentBeginOverlap(XCollision)
  (params (OverlappedComponent :type Primitive%20Component%20Object%20Reference) (OtherActor :type Actor%20Object%20Reference) (OtherComp :type Primitive%20Component%20Object%20Reference) (OtherBodyIndex :type Integer) (bFromSweep :type Boolean) (SweepResult :type Hit%20Result%20Structure%20%28by%20ref%29))
  ;[1 1 1] X
  (bind _asbp_first_person_controller (Utilities|Casting|CastToBP_FirstPersonController OtherActor))
  (Variables|/Game/Character/BP_FirstPersonController.BP_FirstPersonController_C|SetIsPushing? _asbp_first_person_controller true))

(event OnComponentEndOverlap(XCollision)
  (params (OverlappedComponent :type Primitive%20Component%20Object%20Reference) (OtherActor :type Actor%20Object%20Reference) (OtherComp :type Primitive%20Component%20Object%20Reference) (OtherBodyIndex :type Integer))
  ;[1 1 1] X
  (bind _asbp_first_person_controller (Utilities|Casting|CastToBP_FirstPersonController OtherActor))
  (Variables|/Game/Character/BP_FirstPersonController.BP_FirstPersonController_C|SetIsPushing? _asbp_first_person_controller false))

(event OnComponentBeginOverlap(Sphere)
  (params (OverlappedComponent :type Primitive%20Component%20Object%20Reference) (OtherActor :type Actor%20Object%20Reference) (OtherComp :type Primitive%20Component%20Object%20Reference) (OtherBodyIndex :type Integer) (bFromSweep :type Boolean) (SweepResult :type Hit%20Result%20Structure%20%28by%20ref%29))
  ;[1 1 1] Подсветка
  (Utilities|Casting|CastToBP_FirstPersonController OtherActor)
  (Rendering|SetRenderCustomDepth (Variables|Default|GetCube) true))

(event OnComponentEndOverlap(Sphere)
  (params (OverlappedComponent :type Primitive%20Component%20Object%20Reference) (OtherActor :type Actor%20Object%20Reference) (OtherComp :type Primitive%20Component%20Object%20Reference) (OtherBodyIndex :type Integer))
  ;[1 1 1] Подсветка
  (Utilities|Casting|CastToBP_FirstPersonController OtherActor)
  (Rendering|SetRenderCustomDepth (Variables|Default|GetCube) false))

(event EventTick
  (params (DeltaSeconds :type Float%20%28single-precision%29))
  (bind _asbp_first_person_controller (Utilities|Casting|CastToBP_FirstPersonController (Game|GetPlayerCharacter 0)))
  (if (<= (Variables|/Game/Character/BP_FirstPersonController.BP_FirstPersonController_C|GetHealth _asbp_first_person_controller) 0.0)
    (Physics|SetPhysicsLinearVelocity (Variables|Default|GetCube) "0, 0, 0" false "None")
    (Transformation|SetWorldLocation (Variables|Default|GetCube) (Variables|Default|Getstart_vec) false false)))

(event EventBeginPlay
  (Physics|SetSimulatePhysics (Variables|Default|GetCube) true)
  (Variables|Default|Setstart_vec (Transformation|GetWorldLocation (Variables|Default|GetCube))))

(fn ConstructionScript)