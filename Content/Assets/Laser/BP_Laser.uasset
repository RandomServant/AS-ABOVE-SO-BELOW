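; BP_Laser is a laser hazard that damages the player and zeroes a vacuum cleaner's HP on contact.
; A Box overlap with BP_FirstPersonController starts a delayed loop that calls GetHit and subtracts Health at a short interval while the shared Overlap flag holds.
; An overlapping BP_VacuumCleaner has its HP set straight to zero.
; Any end overlap clears the flag, which stops the damage loop at its next check.
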(event OnComponentBeginOverlap(Box)
  (params (OverlappedComponent :type Primitive%20Component%20Object%20Reference) (OtherActor :type Actor%20Object%20Reference) (OtherComp :type Primitive%20Component%20Object%20Reference) (OtherBodyIndex :type Integer) (bFromSweep :type Boolean) (SweepResult :type Hit%20Result%20Structure%20%28by%20ref%29))
  (Variables|Default|Setoverlap true)
  (bind _asbp_first_person_controller (Utilities|Casting|CastToBP_FirstPersonController OtherActor)
    (:then
      (Utilities|FlowControl|Delay 0.2 :!label _label)
      (if (Variables|Default|Getoverlap)
        (Default|GetHit _asbp_first_person_controller)
        (Variables|/Game/Character/BP_FirstPersonController.BP_FirstPersonController_C|SetHealth _asbp_first_person_controller (- (Variables|/Game/Character/BP_FirstPersonController.BP_FirstPersonController_C|GetHealth _asbp_first_person_controller) 1e+01))
        (goto _label)
        (else
          (Variables|Default|Setoverlap false))))
    (:CastFailed
      (bind _asbp_vacuum_cleaner (Utilities|Casting|CastToBP_VacuumCleaner OtherActor))
      (Variables|/Game/VacumCleaner/BP_VacuumCleaner.BP_VacuumCleaner_C|SetHP _asbp_vacuum_cleaner 0.0))))

(event OnComponentEndOverlap(Box)
  (params (OverlappedComponent :type Primitive%20Component%20Object%20Reference) (OtherActor :type Actor%20Object%20Reference) (OtherComp :type Primitive%20Component%20Object%20Reference) (OtherBodyIndex :type Integer))
  (Variables|Default|Setoverlap false))

(fn ConstructionScript)